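; BP_player2 is a player Blueprint that handles basic walk and look controls through Enhanced Input.
; On BeginPlay it adds the IMC_player mapping context to the local subsystem of player controller 0.
; IA_move feeds movement input along the actor's forward and right vectors, with X driving forward and Y driving sideways.
; IA_look passes its axes to controller yaw and pitch input.
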(event `self.ReceiveBeginPlay`
  (`EnhancedInputSubsystemInterface.AddMappingContext` (pcsubsystem `EnhancedInputLocalPlayerSubsystem` (`GameplayStatics.GetPlayerController` 0)) "/Game/IMC_player.IMC_player" 0 (struct)))

(event `EnhancedInput|/Game/IA_move`
  (params (ActionValue :type "Vector2D Structure") (ElapsedSeconds :type "Float (double-precision)") (TriggeredSeconds :type "Float (double-precision)") (InputAction :type "InputAction Object Reference" :default "/Game/IA_move.IA_move"))
  (:`Triggered`
    (`self.AddMovementInput` (`self.GetActorForwardVector`) ActionValue_X)
    (`self.AddMovementInput` (`self.GetActorRightVector`) ActionValue_Y)))

(event `EnhancedInput|/Game/IA_look`
  (params (ActionValue :type "Vector2D Structure") (ElapsedSeconds :type "Float (double-precision)") (TriggeredSeconds :type "Float (double-precision)") (InputAction :type "InputAction Object Reference" :default "/Game/IA_look.IA_look"))
  (:`Triggered`
    (`self.AddControllerPitchInput` ActionValue_Y)
    (`self.AddControllerYawInput` ActionValue_X)))

(fn `UserConstructionScript`)